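; Assault rifle class Blueprint in the Characters folder that provides automatic fire on the shoot input.
; Pressing IA_Shoot fires once immediately, then a looping timer at FireRate repeats Shoot until release clears it.
; Each shot calls both ProjectileBullet and LineTraceBullet, then plays a non-spatial 2D gunshot sound, noted for a 3D replacement in multiplayer.
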(event `Shoot`
  ;[1 1 1] Spawns Projectile based off of the Camera Pitch and Player Yaw Rotations
  (`self.ProjectileBullet`)
  (`self.LineTraceBullet`)
  ;[1 1 1] Change to 3D sound for multiplayer
  (`GameplayStatics.PlaySound2D` "/Game/FX/SoundFX/556_Single_WAV_Quiet.556_Single_WAV_Quiet" 1.0 1.0 0.0 null null))

(event `EnhancedInput|/Game/Blueprints/FirstPerson/Input/Actions/IA_Shoot`
  (params (ActionValue :type Boolean) (ElapsedSeconds :type "Float (double-precision)") (TriggeredSeconds :type "Float (double-precision)") (InputAction :type "InputAction Object Reference" :default "/Game/Blueprints/FirstPerson/Input/Actions/IA_Shoot.IA_Shoot"))
  (:`Started`
    ;[1 1 1] Tap Fire
    (`self.Shoot`)
    ;[1 1 1] Holding Down Fire
    (bind _returnvalue (`KismetSystemLibrary.K2_SetTimerDelegate` (delegate `Shoot`) (`self.FireRate`) true))
    (set `self.Timer` _returnvalue))
  (:`Completed`
    ;[1 1 1] Clear Timer
    (`KismetSystemLibrary.K2_ClearAndInvalidateTimerHandle` (`self.Timer`))))

(fn `UserConstructionScript`
  (`parent.UserConstructionScript`))